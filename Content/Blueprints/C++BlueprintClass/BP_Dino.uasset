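; BP_Dino is a flipbook-based dino character that jumps, slides and can turn big through a power-up.
; Space and S call Jumping and Sliding through DoOnce gates that reset on release, giving one call per press.
; The PowerUp event or E key sets UseBigMode when BigMode is true.
; Tick then raises the sprite and swaps to the big-dino flipbook, otherwise holding the sprite at its lower offset.
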(event `Key|SpaceBar`
  (params (Key :type "Key Structure"))
  (:`Pressed`
    (`/Engine/EditorBlueprintResources/StandardMacros.DoOnce` false :!label _label
      (:`Completed`
        (`self.Jumping`))))
  (:`Released`
    (goto _label :!via `Reset`)))

(event `Key|S`
  (params (Key :type "Key Structure"))
  (:`Pressed`
    (`/Engine/EditorBlueprintResources/StandardMacros.DoOnce` false :!label _label_2
      (:`Completed`
        (`self.Sliding`))))
  (:`Released`
    (goto _label_2 :!via `Reset`)))

(event `PowerUp`
  (if (`self.BigMode`) :!label _label_3
    (set `self.UseBigMode` true)))

(event `Key|E`
  (params (Key :type "Key Structure"))
  (:`Pressed`
    (goto _label_3)))

(event `self.ReceiveTick`
  (params (DeltaSeconds :type "Float (single-precision)"))
  (bind _sprite (`self.Sprite`))
  (if (`self.UseBigMode`)
    (`SceneComponent.K2_SetRelativeLocation` _sprite (0.0 0.0 30.0) false false)
    (`PaperFlipbookComponent.SetFlipbook` _sprite "/Game/Assets/BIGDIno/FB_BigDino.FB_BigDino")
    (else
      (`SceneComponent.K2_SetRelativeLocation` _sprite (0.0 0.0 -7.0) false false))))

(fn `UserConstructionScript`)