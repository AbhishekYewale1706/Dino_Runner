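; Game mode for a dino endless runner that creates the gameplay HUD, runs the power-up meter and handles game over.
; Looping timers fill the meter to enable the dino's BigMode, then drain it once that mode is used and restart charging.
; Tick refreshes coin, distance, time and health text.
; On death it launches the dino upward, disables its input and shows the game-over widget.
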(event `self.ReceiveBeginPlay`
  (bind _returnvalue (`GameplayStatics.GetPlayerController` 0))
  (`|ExecutionSequence`
    (:`then_0`
      ;[0 0.02668 0.15 0.5] Comment
      (bind _returnvalue_2 (`|CreateWidget` "/Game/Blueprints/C++BlueprintClass/HUD/WB_GamePlayHUD.WB_GamePlayHUD_C" _returnvalue))
      (bind _output_get (set `self.As GamePlaye HUD` _returnvalue_2))
      (`UserWidget.AddToViewport` _output_get 0)
      (set `PlayerController.bShowMouseCursor` false _returnvalue)
      (`WidgetBlueprintLibrary.SetInputMode_GameOnly` _returnvalue))
    (:`then_1`
      (`KismetSystemLibrary.Delay` 2.0)
      (`self.PowerUse`))))

(event `StopPowerUpUseTime`
  ;[0.15 0 0 0.5] Power up
  (`KismetSystemLibrary.K2_ClearAndInvalidateTimerHandle` (stale `PowerUse` _returnvalue)))

(event `PowerUse`
  ;[0.15 0 0 0.5] Power up
  (bind _returnvalue (`KismetSystemLibrary.K2_SetTimerDelegate` (delegate `PowerTimeIncrease`) 0.1 true)))

(event `ShowPowerButon`
  ;[0.15 0 0 0.5] Power up
  (`Widget.SetVisibility` (`/Game/Blueprints/C++BlueprintClass/HUD/WB_GamePlayHUD.PowerUpButton` (`self.As GamePlaye HUD`)) "Visible"))

(event `ResetShowPowerButton`
  ;[0.15 0 0 0.5] Power up
  (goto _label :!via `Reset`))

(event `PowerTimeIncrease`
  (bind _asbpdino (`self.AsBPDino`))
  ;[0.15 0 0 0.5] Power up
  (set `self.PowerTime` (`KismetMathLibrary.FClamp` (+ (`self.PowerTime`) 0.2) -0.5 100.5))
  (if (> (`self.PowerTime`) 100.0)
    (`|ExecutionSequence`
      (:`then_0`
        (`/Engine/EditorBlueprintResources/StandardMacros.DoOnce` false :!label _label
          (:`Completed`
            (`self.ShowPowerButon`)
            (`self.ResetHideButton`))))
      (:`then_1`
        (set `Dino.BigMode` true _asbpdino)
        (if (`Dino.UseBigMode` _asbpdino)
          (`self.PowerNotUse`)
          (`self.StopPowerUpUseTime`))))
    (else
      (`ProgressBar.SetPercent` (`/Game/Blueprints/C++BlueprintClass/HUD/WB_GamePlayHUD.PowerUpBar` (`self.As GamePlaye HUD`)) (/ (`self.PowerTime`) 100.0)))))

(event `StopPowerUpTimeNotUse`
  ;[0.15 0 0 0.5] Power up
  (`KismetSystemLibrary.K2_ClearAndInvalidateTimerHandle` (stale `PowerNotUse` _returnvalue)))

(event `PowerNotUse`
  ;[0.15 0 0 0.5] Power up
  (bind _returnvalue (`KismetSystemLibrary.K2_SetTimerDelegate` (delegate `ReducePowerTime`) 0.1 true)))

(event `ResetHideButton`
  ;[0.15 0 0 0.5] Power up
  (goto _label_2 :!via `Reset`))

(event `ReducePowerTime`
  (bind _asbpdino (`self.AsBPDino`))
  ;[0.15 0 0 0.5] Power up
  (set `self.PowerTime` (`KismetMathLibrary.FClamp` (- (`self.PowerTime`) 0.8) -0.5 100.5))
  (if (< (`self.PowerTime`) 0.0)
    (`|ExecutionSequence`
      (:`then_0`
        (`/Engine/EditorBlueprintResources/StandardMacros.DoOnce` false :!label _label_2
          (:`Completed`
            (`self.ResetShowPowerButton`))))
      (:`then_1`
        (set `Dino.BigMode` false _asbpdino)
        (set `Dino.UseBigMode` false _asbpdino)
        (`KismetSystemLibrary.Delay` 2.0)
        (`self.PowerUse`)
        (`self.StopPowerUpTimeNotUse`)))
    (else
      (`ProgressBar.SetPercent` (`/Game/Blueprints/C++BlueprintClass/HUD/WB_GamePlayHUD.PowerUpBar` (`self.As GamePlaye HUD`)) (/ (`self.PowerTime`) 100.0)))))

(event `self.ReceiveTick`
  (params (DeltaSeconds :type "Float (single-precision)"))
  (bind _returnvalue (`GameplayStatics.GetPlayerController` 0))
  (bind _asbpdino (`self.AsBPDino`))
  (bind _asbpdino_2 (`self.AsBPDino`)
    (:`then`
      (if (`Dino.IsDead` _asbpdino_2)
        ;[0 0.02018 0.15 0.5] Comment
        (`/Engine/EditorBlueprintResources/StandardMacros.DoOnce` false
          (:`Completed`
            (`Character.LaunchCharacter` _asbpdino (0.0 0.0 5000.0) false false)
            (`self.DisableInput` _asbpdino null)
            (`KismetSystemLibrary.Delay` 0.5)
            (set `PlayerController.bShowMouseCursor` true _returnvalue)
            (bind _returnvalue_2 (`|CreateWidget` "/Game/Blueprints/C++BlueprintClass/HUD/WB_GameOverHUD.WB_GameOverHUD_C" _returnvalue))
            (`UserWidget.AddToViewport` _returnvalue_2 0)
            (`WidgetBlueprintLibrary.SetInputMode_GameAndUIEx` _returnvalue _returnvalue_2)))
        (else
          (`self.UI Update`))))
    (:`else`)))

(fn `UI Update`
  (set `TextBlock.Text` (`KismetTextLibrary.Conv_IntToText` (`self.Coin`)) (`/Game/Blueprints/C++BlueprintClass/HUD/WB_GamePlayHUD.CoinText` (`self.As GamePlaye HUD`)))
  (set `TextBlock.Text` (`KismetTextLibrary.Conv_StringToText` (`KismetStringLibrary.Concat_StrStr` (`KismetTextLibrary.Conv_TextToString` (`KismetTextLibrary.Conv_IntToText` (`KismetMathLibrary.Round` (`self.DistanceTravel`)))) "m")) (`/Game/Blueprints/C++BlueprintClass/HUD/WB_GamePlayHUD.DistanceText` (`self.As GamePlaye HUD`)))
  (set `TextBlock.Text` (`KismetTextLibrary.Conv_StringToText` (`KismetStringLibrary.Concat_StrStr` (`KismetTextLibrary.Conv_TextToString` (`KismetTextLibrary.Conv_IntToText` (`KismetMathLibrary.Round` (`self.Time`)))) "s")) (`/Game/Blueprints/C++BlueprintClass/HUD/WB_GamePlayHUD.TimeText` (`self.As GamePlaye HUD`)))
  (set `TextBlock.Text` (`KismetTextLibrary.Conv_StringToText` (`KismetStringLibrary.Concat_StrStr` "x" (`KismetStringLibrary.Conv_IntToString` (`KismetMathLibrary.Round` (`Dino.Health` (`self.AsBPDino`)))))) (`/Game/Blueprints/C++BlueprintClass/HUD/WB_GamePlayHUD.Dinotext` (`self.As GamePlaye HUD`))))

(fn `UserConstructionScript`)